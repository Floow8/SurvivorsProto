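; BP_Chicken is a timed healing pickup that calls HealHalf on the player's BP_PlayerStats component and expires if left uncollected.
; Tick polls distance to the player instead of using overlap, then plays a sound, spawns a BP_PoofFX burst, heals and destroys the actor.
; It also carries an InitChest function that stores a perk count and enlarges the mesh for higher counts, unused by the pickup logic.
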(event `self.ReceiveBeginPlay`
  (`self.SetLifeSpan` 45.0))

(event `self.ReceiveTick`
  (params (DeltaSeconds :type "Float (single-precision)"))
  (if (< (`KismetMathLibrary.VSize` (- (`self.K2_GetActorLocation` (`GameplayStatics.GetPlayerCharacter` 0)) (`self.K2_GetActorLocation`))) 110.0)
    (`GameplayStatics.PlaySound2D` "/Game/Survivors/Audio/powerUp1.powerUp1" 0.5 1.0 0.0 null null)
    (bind _returnvalue (`|SpawnActorFromClass` "/Game/Survivors/FX/BP_PoofFX.BP_PoofFX_C" (`KismetMathLibrary.MakeTransform` (`self.K2_GetActorLocation`) (`KismetMathLibrary.MakeRotator` 0.0)) "AlwaysSpawn" "MultiplyWithRoot" null null))
    (bind _asbp_poof_fx (cast `/Game/Survivors/FX/BP_PoofFX` _returnvalue))
    (`/Game/Survivors/FX/BP_PoofFX.InitPoof` _asbp_poof_fx 0.3 3.0)
    (`/Game/Survivors/BP_PlayerStats.HealHalf` (`self.GetComponentByClass` (`GameplayStatics.GetPlayerCharacter` 0) "/Game/Survivors/BP_PlayerStats.BP_PlayerStats_C"))
    (`self.K2_DestroyActor` self)))

(fn `InitChest`
  (params (Perks :type Integer))
  (set `self.PerkCount` Perks)
  (if (>= Perks 3)
    (`SceneComponent.SetRelativeScale3D` (`self.GetComponentByClass` self "/Script/Engine.StaticMeshComponent") (`KismetMathLibrary.MakeVector` 1.2 1.2 1.0))))

(fn `UserConstructionScript`)
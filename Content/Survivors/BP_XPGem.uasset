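; XP pickup gem for a Survivors-style game that expires after a minute if not collected.
; InitGem stores the XP value and derives capped scale and tiered material tint from it; the Kind input is unused.
; Tick spins the gem, pulls it toward the player within BP_PlayerStats' magnet radius, then at close range spawns a poof, grants XP and destroys itself.
; Collection uses distance checks rather than overlaps; older disconnected logic remains in both graphs.
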(event `self.ReceiveBeginPlay`
  (`self.SetLifeSpan` 60.0))

(event `self.ReceiveTick`
  (params (DeltaSeconds :type "Float (single-precision)"))
  (bind _returnvalue (`GameplayStatics.GetPlayerCharacter` 0))
  (bind _returnvalue_2 (`self.K2_GetActorLocation`))
  (bind _returnvalue_3 (`self.GetComponentByClass` _returnvalue "/Game/Survivors/BP_PlayerStats.BP_PlayerStats_C"))
  (bind _returnvalue_4 (`KismetMathLibrary.VSize` (- (`self.K2_GetActorLocation` _returnvalue) _returnvalue_2)))
  (`self.K2_AddActorLocalRotation` (`KismetMathLibrary.MakeRotator` 0.0 0.0 (* 240.0 DeltaSeconds)))
  (bind _returnvalue_5 (`/Game/Survivors/BP_PlayerStats.GetMagnetValue` _returnvalue_3))
  (if (< _returnvalue_4 _returnvalue_5)
    (`self.K2_SetActorLocation` (+ _returnvalue_2 (* (`KismetMathLibrary.Normal` (- (`self.K2_GetActorLocation` _returnvalue) _returnvalue_2)) (* 900.0 DeltaSeconds)))))
  (if (< _returnvalue_4 90.0)
    (bind _returnvalue_6 (`|SpawnActorFromClass` "/Game/Survivors/FX/BP_PoofFX.BP_PoofFX_C" (`KismetMathLibrary.MakeTransform` (`self.K2_GetActorLocation`)) "AlwaysSpawn" "MultiplyWithRoot" null null))
    (`/Game/Survivors/FX/BP_PoofFX.InitPoof` _returnvalue_6 0.12 1.2)
    (`/Game/Survivors/BP_PlayerStats.AddXP` _returnvalue_3 (`self.XPValue`))
    (`self.K2_DestroyActor` self)))

(fn `InitGem`
  (params (Value :type "Float (double-precision)") (Kind :type Integer))
  (set `self.XPValue` Value)
  (`self.SetActorScale3D` (`KismetMathLibrary.MakeVector` (select `bool` (> (+ 0.8 (* 0.02 Value)) 1.3) :`false` (+ 0.8 (* 0.02 Value)) :`true` 1.3) (select `bool` (> (+ 0.8 (* 0.02 Value)) 1.3) :`false` (+ 0.8 (* 0.02 Value)) :`true` 1.3) (select `bool` (> (+ 0.8 (* 0.02 Value)) 1.3) :`false` (+ 0.8 (* 0.02 Value)) :`true` 1.3)))
  (bind _asstatic_mesh_component (cast `StaticMeshComponent` (`self.GetComponentByClass` self "/Script/Engine.StaticMeshComponent")))
  (`MeshComponent.SetVectorParameterValueOnMaterials` _asstatic_mesh_component "Tint" (`KismetMathLibrary.Conv_LinearColorToVector` (make `LinearColor` (select `bool` (< Value 6.0) :`false` (select `bool` (< Value 15.0) :`false` (select `bool` (< Value 30.0) :`false` 2.2 :`true` 3.0) :`true` 0.3) :`true` 0.25) (select `bool` (< Value 6.0) :`false` (select `bool` (< Value 15.0) :`false` (select `bool` (< Value 30.0) :`false` 0.3 :`true` 1.1) :`true` 3.0) :`true` 0.7) (select `bool` (< Value 6.0) :`false` (select `bool` (< Value 15.0) :`false` (select `bool` (< Value 30.0) :`false` 3.0 :`true` 0.15) :`true` 0.5) :`true` 3.0) 1.0))))

(fn `UserConstructionScript`)
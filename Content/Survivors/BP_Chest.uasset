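; BP_Chest is a pickup that grants random player upgrades and expires if not collected in time.
; Tick checks distance to the player instead of using overlap, then plays a sound, spawns a BP_PoofFX and destroys the chest.
; Collection applies one to three random upgrades through BP_PlayerStats, based on the PerkCount set by InitChest.
; InitChest also enlarges the mesh for chests with three or more perks.
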(event `self.ReceiveBeginPlay`
  (`self.SetLifeSpan` 45.0))

(event `self.ReceiveTick`
  (params (DeltaSeconds :type "Float (single-precision)"))
  (bind _returnvalue (`GameplayStatics.GetPlayerCharacter` 0))
  (bind _returnvalue_2 (`self.GetComponentByClass` _returnvalue "/Game/Survivors/BP_PlayerStats.BP_PlayerStats_C"))
  (if (< (`KismetMathLibrary.VSize` (- (`self.K2_GetActorLocation` _returnvalue) (`self.K2_GetActorLocation`))) 110.0)
    (`GameplayStatics.PlaySound2D` "/Game/Survivors/Audio/powerUp1.powerUp1" 0.8 1.0 0.0 null null)
    (bind _returnvalue_3 (`|SpawnActorFromClass` "/Game/Survivors/FX/BP_PoofFX.BP_PoofFX_C" (`KismetMathLibrary.MakeTransform` (`self.K2_GetActorLocation`)) "AlwaysSpawn" "MultiplyWithRoot" null null))
    (`/Game/Survivors/FX/BP_PoofFX.InitPoof` _returnvalue_3 0.6 6.0)
    (`/Game/Survivors/BP_PlayerStats.ApplyUpgrade` _returnvalue_2 (`KismetMathLibrary.RandomIntegerInRange` 0 8))
    (if (>= (`self.PerkCount`) 2)
      (`/Game/Survivors/BP_PlayerStats.ApplyUpgrade` _returnvalue_2 (`KismetMathLibrary.RandomIntegerInRange` 0 8)))
    (if (>= (`self.PerkCount`) 3)
      (`/Game/Survivors/BP_PlayerStats.ApplyUpgrade` _returnvalue_2 (`KismetMathLibrary.RandomIntegerInRange` 0 8)))
    (`self.K2_DestroyActor` self)))

(fn `InitChest`
  (params (Perks :type Integer))
  (set `self.PerkCount` Perks)
  (if (>= Perks 3)
    (`SceneComponent.SetRelativeScale3D` (`self.GetComponentByClass` self "/Script/Engine.StaticMeshComponent") (`KismetMathLibrary.MakeVector` 1.2 1.2 1.0))))

(fn `UserConstructionScript`)
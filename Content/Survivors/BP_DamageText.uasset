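; BP_DamageText is a short-lived floating damage number actor that rises and then destroys itself.
; BeginPlay sets a sub-second lifespan and turns the actor to face the player camera once, while Tick moves it upward at constant speed.
; ShowDamage writes the rounded value into the WBP_DamageNumber held by its NumWidget component and tints the text gold for critical hits.
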(event `self.ReceiveBeginPlay`
  (bind _returnvalue (`PlayerCameraManager.GetCameraRotation` (`GameplayStatics.GetPlayerCameraManager` 0)))
  (`self.SetLifeSpan` 0.9)
  (`self.K2_SetActorRotation` (`KismetMathLibrary.MakeRotator` 0.0 (- 0.0 (.pitch _returnvalue)) (+ (.yaw _returnvalue) 180.0))))

(event `self.ReceiveTick`
  (params (DeltaSeconds :type "Float (single-precision)"))
  (`self.K2_AddActorWorldOffset` (`KismetMathLibrary.MakeVector` 0.0 0.0 (* 120.0 DeltaSeconds))))

(fn `ShowDamage`
  (params (Value :type "Float (double-precision)") (IsCrit :type Boolean))
  (bind _aswbp_damage_number (cast `/Game/Survivors/UI/WBP_DamageNumber` (`WidgetComponent.GetUserWidgetObject` (`self.NumWidget`))))
  (`TextBlock.SetText` (`/Game/Survivors/UI/WBP_DamageNumber.DamageText` _aswbp_damage_number) (`KismetTextLibrary.Conv_IntToText` (`KismetMathLibrary.Round` Value)))
  (if IsCrit
    (set `TextBlock.ColorAndOpacity` (make `SlateColor` (make `LinearColor` 1.0 0.82 0.05 1.0)) (`/Game/Survivors/UI/WBP_DamageNumber.DamageText` _aswbp_damage_number))))

(fn `UserConstructionScript`)
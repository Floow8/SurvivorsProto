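; BP_Prop is a scenery prop actor for the Survivors game that can appear as a green tree, orange tree, bush or mushroom.
; InitProp takes a Kind index and sets the matching material and X/Y scale on the actor's static mesh component, leaving Z at one.
; All variants share that one mesh component, and the event graph and construction script are empty.
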(fn `InitProp`
  (params (Kind :type Integer))
  (bind _returnvalue (`self.GetComponentByClass` self "/Script/Engine.StaticMeshComponent"))
  (switch `int` Kind
    (:`0`
      (`PrimitiveComponent.SetMaterial` _returnvalue 0 "/Game/Survivors/Sprites/MI_S_TreeGreen.MI_S_TreeGreen")
      (`SceneComponent.SetRelativeScale3D` _returnvalue (`KismetMathLibrary.MakeVector` 1.9 1.9 1.0)))
    (:`1`
      (`PrimitiveComponent.SetMaterial` _returnvalue 0 "/Game/Survivors/Sprites/MI_S_TreeOrange.MI_S_TreeOrange")
      (`SceneComponent.SetRelativeScale3D` _returnvalue (`KismetMathLibrary.MakeVector` 1.8 1.8 1.0)))
    (:`2`
      (`PrimitiveComponent.SetMaterial` _returnvalue 0 "/Game/Survivors/Sprites/MI_S_Bush.MI_S_Bush")
      (`SceneComponent.SetRelativeScale3D` _returnvalue (`KismetMathLibrary.MakeVector` 1.2 1.2 1.0)))
    (:`3`
      (`PrimitiveComponent.SetMaterial` _returnvalue 0 "/Game/Survivors/Sprites/MI_S_Mushroom.MI_S_Mushroom")
      (`SceneComponent.SetRelativeScale3D` _returnvalue (`KismetMathLibrary.MakeVector` 0.9 0.9 1.0)))))

(fn `UserConstructionScript`)
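; BP_PoofFX is a short-lived poof effect actor that destroys itself a fraction of a second after BeginPlay.
; BeginPlay sets a default start scale and growth rate, and InitPoof lets a caller override both.
; Tick grows the scale linearly over time and applies it to the static mesh's X and Y, keeping Z fixed, so it spreads flat.
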(event `self.ReceiveBeginPlay`
  (`self.SetLifeSpan` 0.3)
  (set `self.S` 0.3)
  (set `self.Grow` 3.0))

(event `self.ReceiveTick`
  (params (DeltaSeconds :type "Float (single-precision)"))
  (set `self.S` (+ (`self.S`) (* (`self.Grow`) DeltaSeconds)))
  (`SceneComponent.SetRelativeScale3D` (`self.GetComponentByClass` self "/Script/Engine.StaticMeshComponent") (`KismetMathLibrary.MakeVector` (`self.S`) (`self.S`) 1.0)))

(fn `InitPoof`
  (params (S0 :type "Float (double-precision)") (GrowRate :type "Float (double-precision)"))
  (set `self.S` S0)
  (set `self.Grow` GrowRate))

(fn `UserConstructionScript`)